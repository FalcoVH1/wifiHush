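; BP_Player is a player character with single-axis movement, variable-height jumping and a pogo bounce, driven by Enhanced Input.
; BeginPlay adds the input mapping context and sets the jump hold limit, so holding jump controls height.
; Movement follows the control rotation's forward vector, scaled by input and max walk speed.
; The pogo input launches the character upward, overriding vertical velocity, when its Box overlaps a BP_PogoActor.
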(event `self.ReceiveBeginPlay`
  (bind _asplayer_controller (cast `PlayerController` (`self.GetController`)))
  (`EnhancedInputSubsystemInterface.AddMappingContext` (pcsubsystem `EnhancedInputLocalPlayerSubsystem` _asplayer_controller) "/Game/IMC_Player.IMC_Player" 0 (struct))
  (set `self.JumpMaxHoldTime` (`self.VariableJumpHeightDuration`)))

(event `EnhancedInput|/Game/IA_Move`
  (params (ActionValue :type "Float (double-precision)") (ElapsedSeconds :type "Float (double-precision)") (TriggeredSeconds :type "Float (double-precision)") (InputAction :type "InputAction Object Reference" :default "/Game/IA_Move.IA_Move"))
  (:`Triggered`
    (`self.AddMovementInput` (`KismetMathLibrary.GetForwardVector` (`self.GetControlRotation`)) (* ActionValue (`CharacterMovementComponent.MaxWalkSpeed` (`self.CharacterMovement`))))))

(event `EnhancedInput|/Game/IA_Jump`
  (params (ActionValue :type Boolean) (ElapsedSeconds :type "Float (double-precision)") (TriggeredSeconds :type "Float (double-precision)") (InputAction :type "InputAction Object Reference" :default "/Game/IA_Jump.IA_Jump"))
  (:`Triggered`
    (`self.Jump`))
  (:`Completed`
    (`self.StopJumping`)))

(event `EnhancedInput|/Game/IA_Pogo`
  (params (ActionValue :type Boolean) (ElapsedSeconds :type "Float (double-precision)") (TriggeredSeconds :type "Float (double-precision)") (InputAction :type "InputAction Object Reference" :default "/Game/IA_Pogo.IA_Pogo"))
  (:`Triggered`
    (for _ (`PrimitiveComponent.GetOverlappingActors` (`self.Box`) "/Game/Obstacles/BP_PogoActor.BP_PogoActor_C")
      (`self.LaunchCharacter` (0.0 0.0 750.0) false true))))

(fn `UserConstructionScript`)